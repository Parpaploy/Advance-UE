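; Timeline Blueprint that moves two cube components in sequence when play begins.
; The CubeMoveTo timeline lerps Cube from its cached world location to MoveToLocation, teleport and sweep disabled.
; When it finishes, a second timeline lerps Cube1 from SelfLocation0 to MoveToLocation0.
; Cube1's current location is written to SelfLocation, so the second lerp's start, SelfLocation0, is never set in this graph.
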(event EventBeginPlay
  (Variables|Default|SetSelfLocation (Transformation|GetWorldLocation (Variables|Default|GetCube)))
  (bind _time (Timeline|CubeMoveTo Play)
    (:Update
      (Transformation|SetWorldLocation (Variables|Default|GetCube) (Math|Vector|Lerp(Vector) (Variables|Default|GetSelfLocation) (Variables|Default|GetMoveToLocation) _time) false false))
    (:Finished
      (Variables|Default|SetSelfLocation (Transformation|GetWorldLocation (Variables|Default|GetCube1)))
      (bind _time_2 (Timeline|Timeline Play)
        (:Update
          (Transformation|SetWorldLocation (Variables|Default|GetCube1) (Math|Vector|Lerp(Vector) (Variables|Default|GetSelfLocation_0) (Variables|Default|GetMoveToLocation_0) _time_2) false false))))))

(fn ConstructionScript)