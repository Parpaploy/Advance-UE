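; T2Door_BP1 is a sliding door that stays locked while its referenced MyKey object is valid, printing "No Key".
; Box begin and end overlaps share one check; once MyKey is invalid, a FlipFlop alternates between opening and delayed closing.
; A Timeline drives a relative-location lerp to slide Door along X, reversing after a short delay to close.
; A disconnected branch that sets HasKey never runs.
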(event OnComponentBeginOverlap(Box)
  (params (OverlappedComponent :type Primitive%20Component%20Object%20Reference) (OtherActor :type Actor%20Object%20Reference) (OtherComp :type Primitive%20Component%20Object%20Reference) (OtherBodyIndex :type Integer) (bFromSweep :type Boolean) (SweepResult :type Hit%20Result%20Structure%20%28by%20ref%29))
  (if (not (Utilities|IsValid (Variables|Default|GetMyKey)))
    (Utilities|FlowControl|FlipFlop
      (:A
        (bind _speed (Timeline|Timeline Play)
          (:Update
            (Transformation|SetRelativeLocation (Variables|Default|GetDoor) (Math|Vector|Lerp(Vector) "0, 0, 0" "300.000000,0.000000,0.000000" _speed) false false))))
      (:B
        (Utilities|FlowControl|Delay 3.0)
        (Timeline|Timeline Reverse)))
    (else
      (Development|PrintString "No Key"))))

(event OnComponentEndOverlap(Box)
  (params (OverlappedComponent :type Primitive%20Component%20Object%20Reference) (OtherActor :type Actor%20Object%20Reference) (OtherComp :type Primitive%20Component%20Object%20Reference) (OtherBodyIndex :type Integer))
  (if (not (Utilities|IsValid (Variables|Default|GetMyKey)))
    (Utilities|FlowControl|FlipFlop
      (:A
        (bind _speed (Timeline|Timeline Play)
          (:Update
            (Transformation|SetRelativeLocation (Variables|Default|GetDoor) (Math|Vector|Lerp(Vector) "0, 0, 0" "300.000000,0.000000,0.000000" _speed) false false))))
      (:B
        (Utilities|FlowControl|Delay 3.0)
        (Timeline|Timeline Reverse)))
    (else
      (Development|PrintString "No Key"))))

(event EventTick
  (params (DeltaSeconds :type Float%20%28single-precision%29)))

(fn ConstructionScript)