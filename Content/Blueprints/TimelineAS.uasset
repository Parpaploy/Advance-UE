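; TimelineAS is a Blueprint that animates a machine start-up: a lever moves, then a fan and motor rotate.
; On BeginPlay a timeline lerps the lever's relative rotation to its target along the shortest path.
; When it finishes, a Sequence starts separate fan and motor timelines, each lerping its mesh between start and end rotators without the shortest-path option.
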(event EventBeginPlay
  ;[1 0.722 0.7822] Lever
  (bind _time (Timeline|Timeline Play)
    (:Update
      (Transformation|SetRelativeRotation (Variables|Default|GetLever) (Math|Rotator|Lerp(Rotator) (Variables|Default|GetLeverRotation) (Variables|Default|GetLeverMoveToRotation) _time true) false false))
    (:Finished
      (Utilities|FlowControl|Sequence
        (:then_0
          ;[0.6892 0.7951 1] FanSpin
          (bind _timefan (Timeline|FanTimeline Play)
            (:Update
              (Transformation|SetRelativeRotation (Variables|Default|GetS_Rusty_Radiator_Fan_wcljdev_lod3_Var1) (Math|Rotator|Lerp(Rotator) (Variables|Default|GetFanRotation) (Variables|Default|GetFanMoveToRotation) _timefan) false false))))
        (:then_1
          ;[0.6746 1 0.7278] Motor
          (bind _timemotor (Timeline|MotorTimeline Play)
            (:Update
              (Transformation|SetRelativeRotation (Variables|Default|GetMotor) (Math|Rotator|Lerp(Rotator) (Variables|Default|GetMotorRotationFirst) (Variables|Default|GetMotorRotationEnd) _timemotor) false false))))))))

(fn ConstructionScript)